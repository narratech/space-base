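; Manager actor that finds the BP_Spaceship and spawns asteroids in its path as it travels.
; On BeginPlay it seeds an initial field along the ship's forward vector from world origin.
; Each tick it spawns another ahead along its own forward vector once the ship's distance from origin grows past a threshold.
; Asteroids get random rotation, scale and Y/Z offset, with a random chance of no offset.
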(event `self.ReceiveBeginPlay`
  ;[0.03 0.03 0.03] Event Begin Play
  (`self.AssignSpaceship`)
  (`self.SpawnInitialAsteroids`))

(event `self.ReceiveTick`
  (params (DeltaSeconds :type "Float (single-precision)"))
  ;[0.03 0.03 0.03] Event Tick
  (`self.SpawnAsteroids`))

(fn `UserConstructionScript`)