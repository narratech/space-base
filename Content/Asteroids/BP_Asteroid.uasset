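; Spinning asteroid actor that lasers can shoot down, showing one random mesh and growing in on spawn.
; Scale-based health drops per laser hit, flashing emissive on a dynamic material via timeline.
; At zero health it updates the Spaceship's asteroid count, spawns explosion VFX with camera shake, and destroys itself.
; Tick also silently destroys it once left behind, judged by comparing squared distances of ship and asteroid from world origin.
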(event `self.ReceiveBeginPlay`
  ;[0.03 0.03 0.03] Event Begin Play
  (`self.Set Initial Mesh Visibility`)
  (`self.SetRandomRotationAxis`)
  (`|ExecutionSequence`
    (:`then_0`
      (bind (_direction _scale) (`Timeline|Timeline` :!via `PlayFromStart`)
        (:`Update`
          (`SceneComponent.SetRelativeScale3D` (`self.Art`) (`KismetMathLibrary.Conv_DoubleToVector` _scale)))))
    (:`then_1`
      (`self.SetupHealth`))))

(event `self.ReceiveTick`
  (params (DeltaSeconds :type "Float (single-precision)"))
  ;[0.03 0.03 0.03] Event Tick
  (`self.UpdateRotation`)
  (`self.CheckForDestroyWhenBehindSpaceship`))

(event `self.ReceiveHit`
  (params (MyComp :type "PrimitiveComponent Object Reference") (Other :type "Actor Object Reference") (OtherComp :type "PrimitiveComponent Object Reference") (bSelfMoved :type Boolean) (HitLocation :type "Vector Structure") (HitNormal :type "Vector Structure") (NormalImpulse :type "Vector Structure") (Hit :type "HitResult Structure (by ref)"))
  ;[0.03 0.03 0.03] Event Hit
  (cast `/Game/LaserWeapon/BP_LaserProjectile` Other)
  (bind _output_get (set `self.health` (- (`self.health`) 1.0)))
  (if (<= _output_get 0.0)
    (`self.OnAsteroidDestroyed`)
    (`self.DestroyOnHealthDepleted`)
    (else
      (`self.OnAsteroidDamaged`)
      (bind (_direction _value) (`Timeline|DamageFlash` :!via `PlayFromStart`)
        (:`Update`
          (`MaterialInstanceDynamic.SetScalarParameterValue` (`self.AsteroidMaterial`) "Emissive" _value))))))

(event `OnAsteroidDamaged`
  ;[0.03 0.03 0.03] Health Events
)

(event `OnAsteroidDestroyed`
  (bind _spaceship (`self.spaceship`))
  ;[0.03 0.03 0.03] Health Events
  (`/Game/Spaceship/BP_Spaceship.AsteroidSub` _spaceship)
  (`/Game/Spaceship/BP_Spaceship.AsteroidCount` _spaceship))

(fn `UserConstructionScript`)